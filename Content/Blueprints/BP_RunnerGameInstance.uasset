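; Game instance for a runner game that stores and ranks the leaderboard scores.
; AddNewScore wraps a name and score in a new BP_LeaderboardData object, appends it to the LeaderboardData array and re-sorts.
; SortLeaderboardArray bubble-sorts highest score first, shrinking the pass range each time and clamping the neighbor index, then prints a debug message.
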(fn `AddNewScore`
  (params (Name :type String) (Score :type "Float (double-precision)"))
  (bind _returnvalue (`|GenericCreateObject` "/Game/Blueprints/BP_LeaderboardData.BP_LeaderboardData_C" self))
  (set `/Game/Blueprints/BP_LeaderboardData.Data` (make `/Game/Blueprints/BP_LeaderboardStruct` Name Score) _returnvalue)
  (`KismetArrayLibrary.Array_Add` (`self.LeaderboardData`) _returnvalue)
  (`self.SortLeaderboardArray`))

(fn `SortLeaderboardArray`
  (locals (LastIndex :type Integer) (CurrentIndex :type Integer) (CurrentScoreVal :type "Float (double-precision)"))
  (bind _leaderboarddata (`self.LeaderboardData`))
  (bind _currentindex (`local.CurrentIndex`))
  (bind _currentindex_2 (`local.CurrentIndex`))
  (bind (_data_name _data_score) (break `/Game/Blueprints/BP_LeaderboardStruct` (`/Game/Blueprints/BP_LeaderboardData.Data` (`|GetArrayItem` (`self.LeaderboardData`) _currentindex_2))))
  (bind (_data_name_2 _data_score_2) (break `/Game/Blueprints/BP_LeaderboardStruct` (`/Game/Blueprints/BP_LeaderboardData.Data` (`|GetArrayItem` (`self.LeaderboardData`) (`KismetMathLibrary.Clamp` (+ _currentindex_2 1) 0 (`local.LastIndex`))))))
  (set `local.LastIndex` (`KismetArrayLibrary.Array_LastIndex` _leaderboarddata))
  (for _ _leaderboarddata
    (for _index (range (+ (`local.LastIndex`) 1))
      (set `local.CurrentIndex` _index)
      (bind _output_get (set `local.CurrentScoreVal` _data_score))
      (if (< _output_get _data_score_2)
        (`KismetArrayLibrary.Array_Swap` (`self.LeaderboardData`) _currentindex (+ _currentindex 1))))
    (`/Engine/EditorBlueprintResources/StandardMacros.DecrementInt` (`local.LastIndex`)))
  (`KismetSystemLibrary.PrintString` "Done Sorting Leaderboard" true true (struct :`R` 0.062289 :`G` 1.0 :`A` 1.0)))