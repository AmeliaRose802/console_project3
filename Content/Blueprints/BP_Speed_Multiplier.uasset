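; BP_Speed_Multiplier is a collectible that applies a timed speed multiplier in what appears to be a runner game.
; Its Collected override casts the game mode to BP_RunnerGamemode, passes its Multiplier and Duration variables to SetSpeedMultiplier, then calls the parent Collected.
; If the cast fails, the parent call is skipped as well.
; The event graph holds only disabled default events, so Collected is the only logic added here.
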(fn `Collected`
  (bind _asbp_runner_gamemode (cast `/Game/Blueprints/BP_RunnerGamemode` (`GameplayStatics.GetGameMode`)))
  (`/Game/Blueprints/BP_RunnerGamemode.SetSpeedMultiplier` _asbp_runner_gamemode (`self.Multiplier`) (`self.Duration`))
  (`parent.Collected`))

(fn `UserConstructionScript`
  (`parent.UserConstructionScript`))