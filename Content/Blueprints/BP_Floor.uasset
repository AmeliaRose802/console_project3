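; BP_Floor is a track tile for a runner game that can carry one obstacle and removes itself once passed.
; On BeginPlay, if obstacle spawning is enabled, it spawns a BP_Obstacle at one of three marker points chosen at random.
; When the player overlaps BackTileTrigger, it asks BP_RunnerGamemode for another tile, then destroys itself and its obstacle after a delay.
; GetAttachTransform exposes the AttachPoint transform.
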(event `self.ReceiveBeginPlay`
  (if (`self.bSpawnObstacle`)
    (set `self.ObstacleSpawnTransforms` (`|MakeArray` (`SceneComponent.K2_GetComponentToWorld` (`self.ObstacleSpawn1`)) (`SceneComponent.K2_GetComponentToWorld` (`self.ObstacleSpawn2`)) (`SceneComponent.K2_GetComponentToWorld` (`self.ObstacleSpawn3`))))
    (`self.SpawnObstacle`)))

(event `self.BackTileTrigger.OnComponentBeginOverlap`
  (params (OverlappedComponent :type "PrimitiveComponent Object Reference") (OtherActor :type "Actor Object Reference") (OtherComp :type "PrimitiveComponent Object Reference") (OtherBodyIndex :type Integer) (bFromSweep :type Boolean) (SweepResult :type "HitResult Structure (by ref)"))
  (if (== (`GameplayStatics.GetObjectClass` OtherActor) "/Game/Blueprints/PlayerCharacter.PlayerCharacter_C")
    (bind _asbp_runner_gamemode (cast `/Game/Blueprints/BP_RunnerGamemode` (`GameplayStatics.GetGameMode`)))
    (`/Game/Blueprints/BP_RunnerGamemode.SpawnTile` _asbp_runner_gamemode)
    (`KismetSystemLibrary.Delay` 5.0)
    (if (`self.bSpawnObstacle`)
      (`self.K2_DestroyActor` (`self.Obstacle`)))
    (`self.K2_DestroyActor` self)))

(fn `GetAttachTransform`
  (returns (AttachTransform :type "Transform Structure"))
  (return (`SceneComponent.K2_GetComponentToWorld` (`self.AttachPoint`))))

(fn `SpawnObstacle`
  (bind _returnvalue (`|SpawnActorFromClass` "/Game/Blueprints/BP_Obstacle.BP_Obstacle_C" (`KismetArrayLibrary.Array_Random` (`self.ObstacleSpawnTransforms`)) "Undefined" "OverrideRootScale" null null))
  (set `self.Obstacle` _returnvalue))

(fn `UserConstructionScript`)