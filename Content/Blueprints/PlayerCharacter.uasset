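; Player character that is pushed constantly forward while the player steers it from side to side.
; Each tick, a force on the Mesh drives it along negative world X, scaled by FowardSpeed.
; The SideToSide axis feeds movement input along world Y using Speed.
; HitRock is a placeholder death handler that only prints "Dead Now" and is not called within this Blueprint.
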(event `self.ReceiveTick`
  (params (DeltaSeconds :type "Float (single-precision)"))
  ;[1 1 1] Move Foward
  (`PrimitiveComponent.AddForce` (`self.Mesh`) (`KismetMathLibrary.MakeVector` (* (`self.FowardSpeed`) -1.0)) "None" false))

(event `InputAxis|SideToSide`
  (params (AxisValue :type "Float (single-precision)"))
  ;[1 1 1] Side To Side Movement
  (`self.AddMovementInput` (`KismetMathLibrary.MakeVector` 0.0 (`self.Speed`)) AxisValue))

(event `self.ReceiveActorBeginOverlap`
  (params (OtherActor :type "Actor Object Reference")))

(fn `HitRock`
  (`KismetSystemLibrary.PrintString` "Dead Now"))

(fn `UserConstructionScript`)