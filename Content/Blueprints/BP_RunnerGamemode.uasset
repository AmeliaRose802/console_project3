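; Game mode for an endless runner that spawns floor tiles and tracks score, distance and game over.
; BeginPlay chains initial BP_Floor tiles via attach transforms and starts a looping distance timer, while Tick and coins add score.
; Timed power-ups use delays to boost score or coins, dilate global time, or enable invincibility and coin magnet.
; Obstacle hits without invincibility destroy the player, save the score to the game instance and show the end screen.
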(event `self.ReceiveBeginPlay`
  (set `self.normalGainRate` (`self.ScoreGainRate`))
  (set `self.normalCoinScoreBooster` (`self.CoinScoreBooster`))
  (for _ (range 11)
    (`self.SpawnTile`)
    (bind _asplayer_character (cast `/Game/Blueprints/PlayerCharacter` (`GameplayStatics.GetPlayerCharacter` 0))
      (:`then`
        (set `self.Player` _asplayer_character))
      (:`CastFailed`
        _))
    (`KismetSystemLibrary.K2_SetTimer` null "UpdateDistance" 0.1 true)))

(event `self.ReceiveTick`
  (params (DeltaSeconds :type "Float (single-precision)"))
  (if (not (`self.bGameOver`))
    (set `self.Score` (+ (`self.Score`) (* DeltaSeconds (`self.ScoreGainRate`))))))

(event `GetScoreBooster`
  (params (Multiplier :type "Float (double-precision)") (Time :type "Float (double-precision)"))
  ;[1 1 1] Score booster
  (set `self.ScoreGainRate` (* Multiplier (`self.ScoreGainRate`)))
  (`KismetSystemLibrary.Delay` Time)
  (set `self.ScoreGainRate` (`self.normalGainRate`)))

(event `SetCoinBooster`
  (params (Multiplier :type "Float (double-precision)") (Duration :type "Float (double-precision)"))
  ;[1 1 1] Coin Multiplier
  (set `self.CoinScoreBooster` (* Multiplier (`self.CoinScoreBooster`)))
  (`KismetSystemLibrary.Delay` Duration)
  (set `self.CoinScoreBooster` (`self.normalCoinScoreBooster`)))

(event `SetSpeedMultiplier`
  (params (Multiplier :type "Float (double-precision)") (Duration :type "Float (double-precision)"))
  ;[1 1 1] Set Speed Multiplier
  (`GameplayStatics.SetGlobalTimeDilation` Multiplier)
  (`KismetSystemLibrary.Delay` Duration)
  (`GameplayStatics.SetGlobalTimeDilation` 1.0))

(event `SetUnkillable`
  (params (Duration :type "Float (double-precision)"))
  ;[1 1 1] Invinceable
  (set `self.invincible` true)
  (`KismetSystemLibrary.Delay` Duration)
  (set `self.invincible` false))

(event `SetCoinMag`
  (params (Duration :type "Float (double-precision)"))
  ;[1 1 1] Coin Mag
  (set `self.CoinMagActive` true)
  (`KismetSystemLibrary.Delay` Duration)
  (set `self.CoinMagActive` false))

(fn `AddCoin`
  (params (CoinVal :type "Float (double-precision)"))
  (set `self.Score` (+ (* CoinVal (`self.CoinScoreBooster`)) (`self.Score`))))

(fn `PlayerHitObsticle`
  (bind _returnvalue (`GameplayStatics.GetPlayerController` 0))
  (if (not (`self.invincible`))
    (set `self.bGameOver` true)
    (`self.K2_DestroyActor` (`GameplayStatics.GetPlayerCharacter` 0))
    (`KismetSystemLibrary.PrintString` "Game over now")
    (bind _asbp_runner_game_instance (cast `/Game/Blueprints/BP_RunnerGameInstance` (`GameplayStatics.GetGameInstance`)))
    (bind _asbp_runner_gamemode (cast `/Game/Blueprints/BP_RunnerGamemode` (`GameplayStatics.GetGameMode`)))
    (`/Game/Blueprints/BP_RunnerGameInstance.AddNewScore` _asbp_runner_game_instance "Player" (`/Game/Blueprints/BP_RunnerGamemode.Score` _asbp_runner_gamemode))
    (bind _returnvalue_2 (`|CreateWidget` "/Game/Blueprints/Widgets/WB_EndScreen.WB_EndScreen_C" _returnvalue))
    (`UserWidget.AddToViewport` _returnvalue_2 0)
    (`WidgetBlueprintLibrary.SetInputMode_UIOnlyEx` _returnvalue _returnvalue_2)
    (set `PlayerController.bShowMouseCursor` true _returnvalue)))

(fn `SpawnTile`
  (bind _returnvalue (`LevelGenerator.SpawnFloor` (`self.NextTileSpawnTransform`) "/Game/Blueprints/BP_Floor.BP_Floor_C" self))
  (bind _asbp_floor (cast `/Game/Blueprints/BP_Floor` _returnvalue))
  (bind _attachtransform (`/Game/Blueprints/BP_Floor.GetAttachTransform` _asbp_floor))
  (set `self.NextTileSpawnTransform` _attachtransform))

(fn `UpdateDistance`
  (bind _player (`self.Player`))
  (bind _returnvalue_x (`KismetMathLibrary.BreakVector` (`SceneComponent.K2_GetComponentLocation` (`Character.CapsuleComponent` _player))))
  (`/Engine/EditorBlueprintResources/StandardMacros.IsValid` _player
    (:`Is Valid`
      (set `self.Distance` (`KismetMathLibrary.FTrunc` (`KismetMathLibrary.Distance2D` (`KismetMathLibrary.MakeVector2D` _returnvalue_x) (0.0 0.0)))))))

(fn `UserConstructionScript`)